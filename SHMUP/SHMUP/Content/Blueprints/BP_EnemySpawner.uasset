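; Enemy spawner that gathers every BP_EnemyPath at BeginPlay and runs a looping one-second timer to spawn enemies at them.
; Each spawn event picks a random path, creates a BP_Enemy1 there and starts it moving along that path.
; A delayed branch also spawns a BP_EnemyTurret at whichever path is current when the delay ends, so turrets appear less often than moving enemies.
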(event Custom|Event%20EnemySpawn
  (bind _output_get (Variables|Default|SetCurrentPath (.OutItem (Utilities|Array|Random (Variables|Default|GetAllPaths)))))
  (Utilities|FlowControl|Sequence
    (:then_0
      (Utilities|FlowControl|Delay 5.0)
      (Game|SpawnActorfromClass "/Game/Blueprints/BP_EnemyTurret.BP_EnemyTurret_C" (Math|Transform|MakeTransform (Transformation|GetActorLocation _output_get) "0, 0, 0" "1.000000,1.000000,1.000000") "Undefined" "MultiplyWithRoot" 0 0))
    (:then_1
      (bind _returnvalue (Game|SpawnActorfromClass "/Game/Blueprints/BP_Enemy1.BP_Enemy1_C" (Math|Transform|MakeTransform (Transformation|GetActorLocation _output_get) "0, 0, 0" "1.000000,1.000000,1.000000") "Undefined" "MultiplyWithRoot" 0 1e+02 0 0.2 0))
      (bind _asbp_base_enemy (Utilities|Casting|CastToBP_BaseEnemy _returnvalue)
        (:then
          (Variables|/Game/Blueprints/BP_BaseEnemy.BP_BaseEnemy_C|SetPath _asbp_base_enemy (Variables|Default|GetCurrentPath))
          (Default|StartMovingAlongPath _asbp_base_enemy))
        (:CastFailed
          (Actor|DestroyActor _returnvalue))))))

(event Custom|StartTimer
  (Utilities|Time|SetTimerbyEvent (delegate Custom|Event%20EnemySpawn) 1.0 true))

(event Custom|GetAllPaths
  (bind _outactors (Actor|GetAllActorsOfClass "/Game/Blueprints/BP_EnemyPath.BP_EnemyPath_C"))
  (Variables|Default|SetAllPaths _outactors))

(event EventBeginPlay
  (CallFunction|GetAllPaths)
  (CallFunction|StartTimer))

(fn ConstructionScript)