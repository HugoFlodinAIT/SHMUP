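; Player ship pawn for a shooter, with planar Enhanced Input movement, boost and interpolated roll banking.
; Separate input actions spawn primary, laser, missile, multi, radial and autocannon projectiles, mostly DoOnce/Delay-gated, with FlipFlop alternating primary and missile sides.
; Overlaps subtract AC_Properties damage and update the health widget; death calls GameState respawn and destroys the pawn.
; Shooting-mode switching and widget creation are left unwired.
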(event Custom|Switch%20Shooting%20Mode
  ;[0.15 0.15 0.15 0.5] Fire Mode Switch
  (bind _output_get (Variables|Default|SetShooting%20Mode (Math|Integer|%(Integer) (+ (Variables|Default|GetShooting%20Mode) 1) (+ (Variables|Default|GetMax%20Shooting%20Mode) 1))))
  (Development|PrintString (Utilities|String|ToString(Integer) _output_get)))

(event Input|EnhancedActionEvents|EnhancedInputActionIA_MoveFoward
  (params (ActionValue :type Boolean) (ElapsedSeconds :type Float%20%28double-precision%29) (TriggeredSeconds :type Float%20%28double-precision%29) (InputAction :type Input%20Action%20Object%20Reference :default "/Game/Inputs/IA_MoveFoward.IA_MoveFoward"))
  ;[0.15 0.15 0.15 0.5] Input & Movement
  (Class|PawnMovementComponent|AddInputVector (Variables|Default|GetFloatingPawnMovement) "1.000000,0.000000,0.000000" false))

(event Input|EnhancedActionEvents|EnhancedInputActionIA_MoveBackward
  (params (ActionValue :type Boolean) (ElapsedSeconds :type Float%20%28double-precision%29) (TriggeredSeconds :type Float%20%28double-precision%29) (InputAction :type Input%20Action%20Object%20Reference :default "/Game/Inputs/IA_MoveBackward.IA_MoveBackward"))
  ;[0.15 0.15 0.15 0.5] Input & Movement
  (Class|PawnMovementComponent|AddInputVector (Variables|Default|GetFloatingPawnMovement) "-1.000000,0.000000,0.000000" false))

(event Input|EnhancedActionEvents|EnhancedInputActionIA_FireLaser
  (params (ActionValue :type Boolean) (ElapsedSeconds :type Float%20%28double-precision%29) (TriggeredSeconds :type Float%20%28double-precision%29) (InputAction :type Input%20Action%20Object%20Reference :default "/Game/Inputs/IA_FireLaser.IA_FireLaser"))
  ;[0.15 0 0 0.5] FIre Laser
  (Utilities|FlowControl|DoOnce false :!label _label
    (:Completed
      (bind _returnvalue (Game|SpawnActorfromClass "/Game/Blueprints/Projectiles/BP_Laser.BP_Laser_C" (Math|Transform|MakeTransform (Transformation|GetWorldLocation (Variables|Default|GetFirePrimarySpawn)) "0, 0, 0" "1.000000,1.000000,1.000000") "Undefined" "MultiplyWithRoot" 0 0))
      (Transformation|AttachComponentToComponent _returnvalue (Variables|Default|GetFirePrimarySpawn) "None" "SnapToTarget" "KeepRelative" "KeepRelative" true)
      (Audio|Components|Audio|Play (Variables|Default|GetLaserFire) 0.0)
      (Utilities|FlowControl|Delay 4.0)
      (goto _label Reset))))

(event Input|EnhancedActionEvents|EnhancedInputActionIA_FireAutoCannon
  (params (ActionValue :type Boolean) (ElapsedSeconds :type Float%20%28double-precision%29) (TriggeredSeconds :type Float%20%28double-precision%29) (InputAction :type Input%20Action%20Object%20Reference :default "/Game/Inputs/IA_FireAutoCannon.IA_FireAutoCannon"))
  ;[0.15 0 0 0.5] Fire AutoCannon
  (Utilities|FlowControl|DoOnce false :!label _label
    (:Completed
      (for _index (range 0 (- (Math|Random|RandomIntegerinRange 2 8) 1))
        (Audio|Components|Audio|Play (Variables|Default|GetRadialFire) 0.0)
        (Game|SpawnActorfromClass "/Game/Blueprints/Projectiles/BP_AutoCannon.BP_AutoCannon_C" (Math|Transform|MakeTransform (Transformation|GetWorldLocation (Variables|Default|GetFirePrimarySpawn)) (Math|Rotator|MakeRotator 0.0 0.0 (- (Math|Random|RandomIntegerinRange 2 8) 4)) "1.000000,1.000000,1.000000") "Undefined" "MultiplyWithRoot" 0 (Math|Random|RandomFloatinRange 1e+03 8e+03) true 0)
        (Utilities|FlowControl|Delay 0.01)
        (goto _label Reset)))))

(event Input|EnhancedActionEvents|EnhancedInputActionIA_FireRadial
  (params (ActionValue :type Boolean) (ElapsedSeconds :type Float%20%28double-precision%29) (TriggeredSeconds :type Float%20%28double-precision%29) (InputAction :type Input%20Action%20Object%20Reference :default "/Game/Inputs/IA_FireRadial.IA_FireRadial"))
  ;[0.15 0 0 0.5] Fire Radial
  (Utilities|FlowControl|DoOnce false :!label _label
    (:Completed
      (for _index (range 0 (- (Variables|Default|GetBulletsRadial) 1))
        (Game|SpawnActorfromClass "/Game/Blueprints/Projectiles/BP_Radial.BP_Radial_C" (Math|Transform|MakeTransform (Transformation|GetWorldLocation (Variables|Default|GetFirePrimarySpawn)) (Math|Rotator|MakeRotator 0.0 0.0 (Utilities|Operators|Subtract (* _index 2e+01) (* (Variables|Default|GetBulletsRadial) 1e+01) -1e+01)) "1.000000,1.000000,1.000000") "Undefined" "MultiplyWithRoot" 0 0)
        (Audio|Components|Audio|Play (Variables|Default|GetRadialFire) 0.0)
        (Utilities|FlowControl|Delay 2.0)
        (goto _label Reset)))))

(event Input|EnhancedActionEvents|EnhancedInputActionIA_FireMulti
  (params (ActionValue :type Boolean) (ElapsedSeconds :type Float%20%28double-precision%29) (TriggeredSeconds :type Float%20%28double-precision%29) (InputAction :type Input%20Action%20Object%20Reference :default "/Game/Inputs/IA_FireMulti.IA_FireMulti"))
  ;[0.15 0 0 0.5] Fire Multi
  (Utilities|FlowControl|DoOnce false :!label _label
    (:Completed
      (for _index (range 0 (- (Variables|Default|GetBulletsMulti) 1))
        (Game|SpawnActorfromClass "/Game/Blueprints/Projectiles/BP_Multi.BP_Multi_C" (Math|Transform|MakeTransform (Transformation|GetWorldLocation (Variables|Default|GetFirePrimarySpawn)) (Math|Rotator|MakeRotator 0.0 0.0 (Utilities|Operators|Subtract (* _index 1e+01) (* (Variables|Default|GetBulletsMulti) 5.0) -5.0)) "1.000000,1.000000,1.000000") "Undefined" "MultiplyWithRoot" 0 0)
        (Audio|Components|Audio|Play (Variables|Default|GetMultiFire) 0.0)
        (Utilities|FlowControl|Delay 0.5)
        (goto _label Reset)))))

(event Input|EnhancedActionEvents|EnhancedInputActionIA_MoveLeft
  (params (ActionValue :type Boolean) (ElapsedSeconds :type Float%20%28double-precision%29) (TriggeredSeconds :type Float%20%28double-precision%29) (InputAction :type Input%20Action%20Object%20Reference :default "/Game/Inputs/IA_MoveLeft.IA_MoveLeft"))
  ;[0.15 0.15 0.15 0.5] Input & Movement
  (Class|PawnMovementComponent|AddInputVector (Variables|Default|GetFloatingPawnMovement) "0.000000,-1.000000,0.000000" false))

(event Input|EnhancedActionEvents|EnhancedInputActionIA_MoveRight
  (params (ActionValue :type Boolean) (ElapsedSeconds :type Float%20%28double-precision%29) (TriggeredSeconds :type Float%20%28double-precision%29) (InputAction :type Input%20Action%20Object%20Reference :default "/Game/Inputs/IA_MoveRight.IA_MoveRight"))
  ;[0.15 0.15 0.15 0.5] Input & Movement
  (Class|PawnMovementComponent|AddInputVector (Variables|Default|GetFloatingPawnMovement) "0.000000,1.000000,0.000000" false))

(event Input|EnhancedActionEvents|EnhancedInputActionIA_FireMissile
  (params (ActionValue :type Boolean) (ElapsedSeconds :type Float%20%28double-precision%29) (TriggeredSeconds :type Float%20%28double-precision%29) (InputAction :type Input%20Action%20Object%20Reference :default "/Game/Inputs/IA_FireMissile.IA_FireMissile"))
  (bind _returnvalue (Transformation|GetActorLocation))
  ;[0.15 0 0 0.5] Fire Missile
  (Utilities|FlowControl|Delay 0.75)
  (Utilities|FlowControl|FlipFlop
    (:A
      (Game|SpawnActorfromClass "/Game/Blueprints/Projectiles/BP_Missile.BP_Missile_C" (Math|Transform|MakeTransform _returnvalue "0, 0, 0" "1.000000,1.000000,1.000000") "Undefined" "MultiplyWithRoot" 0 true 0))
    (:B
      (Game|SpawnActorfromClass "/Game/Blueprints/Projectiles/BP_Missile.BP_Missile_C" (Math|Transform|MakeTransform _returnvalue "0, 0, 0" "1.000000,1.000000,1.000000") "Undefined" "MultiplyWithRoot" 0 false 0))))

(event Input|EnhancedActionEvents|EnhancedInputActionIA_FirePrimary
  (params (ActionValue :type Boolean) (ElapsedSeconds :type Float%20%28double-precision%29) (TriggeredSeconds :type Float%20%28double-precision%29) (InputAction :type Input%20Action%20Object%20Reference :default "/Game/Inputs/IA_FirePrimary.IA_FirePrimary"))
  ;[0.15 0.15 0.15 0.5] Fire Mode Switch
  (switch int (Variables|Default|GetShooting%20Mode)))

(event Input|EnhancedActionEvents|EnhancedInputActionIA_Boost
  (params (ActionValue :type Boolean) (ElapsedSeconds :type Float%20%28double-precision%29) (TriggeredSeconds :type Float%20%28double-precision%29) (InputAction :type Input%20Action%20Object%20Reference :default "/Game/Inputs/IA_Boost.IA_Boost"))
  (bind _floatingpawnmovement (Variables|Default|GetFloatingPawnMovement))
  ;[0.15 0.15 0.15 0.5] Input & Movement
  (:Triggered
    (Variables|/Script/Engine.FloatingPawnMovement|SetMaxSpeed _floatingpawnmovement 3e+03))
  (:Completed
    (Variables|/Script/Engine.FloatingPawnMovement|SetMaxSpeed _floatingpawnmovement 2e+03)))

(event Input|EnhancedActionEvents|EnhancedInputActionIA_FirePrimary
  (params (ActionValue :type Boolean) (ElapsedSeconds :type Float%20%28double-precision%29) (TriggeredSeconds :type Float%20%28double-precision%29) (InputAction :type Input%20Action%20Object%20Reference :default "/Game/Inputs/IA_FirePrimary.IA_FirePrimary"))
  (bind _fireprimaryspawn (Variables|Default|GetFirePrimarySpawn))
  (bind _returnvalue (Transformation|GetWorldLocation _fireprimaryspawn))
  ;[0.15 0 0 0.5] Fire Primary
  (Utilities|FlowControl|DoOnce false :!label _label
    (:Completed
      (Utilities|FlowControl|FlipFlop
        (:A
          (Game|SpawnActorfromClass "/Game/Blueprints/Projectiles/BP_Primary.BP_Primary_C" (Math|Transform|MakeTransform (+ _returnvalue "0.000000,100.000000,0.000000") "0, 0, 0" "1.000000,1.000000,1.000000") "Undefined" "MultiplyWithRoot" 0 0)
          (Audio|Components|Audio|Play (Variables|Default|GetPrimaryFire1) 0.0))
        (:B
          (Game|SpawnActorfromClass "/Game/Blueprints/Projectiles/BP_Primary.BP_Primary_C" (Math|Transform|MakeTransform (+ _returnvalue "0.000000,-100.000000,0.000000") "0, 0, 0" "1.000000,1.000000,1.000000") "Undefined" "MultiplyWithRoot" 0 0)
          (Audio|Components|Audio|Play (Variables|Default|GetPrimaryFire) 0.0)))
      (Utilities|FlowControl|Delay 0.1)
      (goto _label Reset))))

(event EventTick
  (params (DeltaSeconds :type Float%20%28single-precision%29))
  (bind _returnvalue (Input|EnhancedActionValues|GetIA_MoveLeft))
  (bind _returnvalue_2 (Input|EnhancedActionValues|GetIA_MoveRight))
  ;[0.15 0.15 0.15 0.5] Banking
  (bind _output_get (Variables|Default|SetDelta%20Seconds DeltaSeconds))
  (bind _output_get_2 (Variables|Default|SetCurrent%20Rotation (Math|Interpolation|FInterpTo (Variables|Default|GetCurrent%20Rotation) (Variables|Default|GetTarget%20Rotation) _output_get 2.0)))
  (Transformation|SetActorRotation (Math|Rotator|MakeRotator (* _output_get_2 35.0) 0.0 0.0))
  (Variables|Default|SetTarget%20Rotation (Math|Float|SelectFloat 0.0 (Math|Float|SelectFloat -1.0 1.0 (Input|EnhancedActionValues|GetIA_MoveLeft)) (or (and _returnvalue _returnvalue_2) (Math|Boolean|NORBoolean _returnvalue_2 _returnvalue)))))

(event EventPossessed
  (params (NewController :type Controller%20Object%20Reference))
  ;[0.15 0.15 0.15 0.5] Input & Movement
  (bind _asplayer_controller (Utilities|Casting|CastToPlayerController NewController))
  (Input|AddMappingContext (PlayerController|LocalPlayerSubsystems|GetEnhancedInputLocalPlayerSubsystem _asplayer_controller) "/Game/Inputs/IMC_PlayerMovement.IMC_PlayerMovement" 0 "(bIgnoreAllPressedKeysUntilRelease=True,bForceImmediately=False,bNotifyUserSettings=False)"))

(event Input|KeyboardEvents|DebugKeyCtrlT
  (params (Key :type Key%20Structure :default "None") (ActionValue :type Input%20Action%20Value%20Structure))
  ;[0.15 0.15 0.15 0.5] Banking
)

(event Collision|EventActorBeginOverlap
  (params (OtherActor :type Actor%20Object%20Reference))
  (Variables|Default|SetCurrentPlayerHealth (- (Variables|Default|GetCurrentPlayerHealth) (Variables|/Game/Blueprints/AC_Properties.AC_Properties_C|GetDamage (Actor|GetComponentbyClass OtherActor "/Game/Blueprints/AC_Properties.AC_Properties_C"))))
  (Default|SetHealth (Variables|Default|GetWDP%20Health) (/ (Variables|Default|GetCurrentPlayerHealth) (Variables|Default|GetMaxPlayerHealth)))
  (if (<= (Variables|Default|GetCurrentPlayerHealth) 0.0)
    (Development|PrintString "DEAD")
    (bind _asbp_game_state (Utilities|Casting|CastToBP_GameState (Game|GetGameState)))
    (Default|SpawnPlayerPawn _asbp_game_state)
    (Actor|DestroyActor)))

(fn ConstructionScript)