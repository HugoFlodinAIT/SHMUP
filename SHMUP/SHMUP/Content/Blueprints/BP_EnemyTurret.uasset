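; Enemy turret that tracks the player pawn, fires at it, and awards score when destroyed.
; A self-calling event with a tiny Delay continuously turns its yaw toward the player.
; BeginPlay starts a randomly delayed loop that spawns player-aimed bullets from three spawn points and plays the Turret component.
; Any overlap subtracts health; at zero it adds points to the WBP_Score widget and destroys itself.
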(event Custom|FacePlayer
  ;[0.15 0.15 0.15 0.5] Look at Player
  (Transformation|SetActorRotation (Math|Rotator|MakeRotator 0.0 0.0 (.yaw (Math|Interpolation|RInterpTo (Transformation|GetActorRotation) (Math|Rotator|FindLookatRotation (Transformation|GetActorLocation) (Transformation|GetActorLocation (Variables|Default|GetChar%20Ref))) (Utilities|Time|GetWorldDeltaSeconds) 1e+03))))
  (Utilities|FlowControl|Delay 0.0001)
  (CallFunction|FacePlayer))

(event EventTick
  (params (DeltaSeconds :type Float%20%28single-precision%29)))

(event EventBeginPlay
  (Utilities|FlowControl|Sequence
    (:then_0
      ;[0.15 0.15 0.15 0.5] Look at Player
      (bind _asbp_player_pawn (Utilities|Casting|CastToBP_PlayerPawn (Game|Player|GetPlayerPawn 0)))
      (Variables|Default|SetChar%20Ref _asbp_player_pawn)
      (CallFunction|FacePlayer))
    (:then_1
      (Utilities|FlowControl|Sequence :!label _label
        (:then_0
          (Game|SpawnActorfromClass "/Game/Blueprints/Projectiles/BP_TurretBullet.BP_TurretBullet_C" (Math|Transform|MakeTransform (Transformation|GetWorldLocation (Variables|Default|Getbulletspawn2)) (Math|Rotator|FindLookatRotation (Transformation|GetActorLocation) (Transformation|GetActorLocation (Variables|Default|GetChar%20Ref))) "1.000000,1.000000,1.000000") "Undefined" "MultiplyWithRoot" 0 0)
          (Utilities|FlowControl|Delay (Math|Random|RandomFloatinRange 1.0 1.5) :!label _label_2)
          (goto _label))
        (:then_1
          ;[0.15 0.15 0.15 0.5] Firing
          (Game|SpawnActorfromClass "/Game/Blueprints/Projectiles/BP_TurretBullet.BP_TurretBullet_C" (Math|Transform|MakeTransform (Transformation|GetWorldLocation (Variables|Default|Getbulletspawn1)) (Math|Rotator|FindLookatRotation (Transformation|GetActorLocation) (Transformation|GetActorLocation (Variables|Default|GetChar%20Ref))) "1.000000,1.000000,1.000000") "Undefined" "MultiplyWithRoot" 0 0)
          (goto _label_2))
        (:then_2
          (Game|SpawnActorfromClass "/Game/Blueprints/Projectiles/BP_TurretBullet.BP_TurretBullet_C" (Math|Transform|MakeTransform (Transformation|GetWorldLocation (Variables|Default|Getbulletspawn3)) (Math|Rotator|FindLookatRotation (Transformation|GetActorLocation) (Transformation|GetActorLocation (Variables|Default|GetChar%20Ref))) "1.000000,1.000000,1.000000") "Undefined" "MultiplyWithRoot" 0 0)
          (goto _label_2))
        (:then_3
          (Audio|Components|Audio|Play (Variables|Default|GetTurret) 0.0))))))

(event Collision|EventActorBeginOverlap
  (params (OtherActor :type Actor%20Object%20Reference))
  ;[0.15 0.15 0.15 0.5] Hit By Enemy
  (|CallParentFunction 0)
  (bind _output_get (Variables|Default|SetHealth (- (Variables|Default|GetHealth) 5e+01)))
  (if (<= _output_get 0.0)
    (bind _foundwidgets (Widget|GetAllWidgetsOfClass "/Game/UI/WBP_Score.WBP_Score_C" false))
    (Default|AddtoScore (Utilities|Array|Get(acopy) _foundwidgets) 50)
    (Actor|DestroyActor)))

(fn ConstructionScript)