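; Base enemy actor that travels along a spline path, with starting health read from its properties component.
; StartMovingAlongPath runs once, driving location through a speed-scaled timeline at constant spline velocity and destroying the actor at the end.
; Overlaps apply a flashing overlay to its static meshes and play a shot sound.
; Any destruction, including reaching the path end, adds the properties' health to player score and may spawn a laser pickup.
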(event Custom|StartMovingAlongPath
  (Utilities|FlowControl|DoOnce false
    (:Completed
      (Components|Timeline|SetPlayRate (Variables|Default|GetTimeline) (Variables|Default|GetSpeed))
      (bind _tracktime (Timeline|Timeline Play)
        (:Update
          (Transformation|SetActorTransform (Math|Transform|MakeTransform (Spline|GetLocationatTime (Variables|/Game/Blueprints/BP_EnemyPath.BP_EnemyPath_C|GetSpline (Variables|Default|GetPath)) _tracktime "World" true) "0, 0, 0" "1.000000,1.000000,1.000000")))
        (:Finished
          (Actor|DestroyActor))))))

(event EventBeginPlay
  (Variables|Default|SetHealth (Variables|/Game/Blueprints/AC_Properties.AC_Properties_C|GetHealth (Variables|Default|GetAC_Properties))))

(event Collision|EventActorBeginOverlap
  (params (OtherActor :type Actor%20Object%20Reference))
  (for _array_element (Actor|GetComponentsByClass "/Script/Engine.StaticMeshComponent")
    (Rendering|Material|SetOverlayMaterial _array_element "/Game/Materials/M_FlashingMaterial.M_FlashingMaterial" :!class /Script/Engine.MeshComponent))
  (Audio|Components|Audio|Play (Variables|Default|GetSciFi_Shot_P2__44__Cue) 0.0))

(event EventEndPlay
  (params (EndPlayReason :type EEndPlayReason%20Enum :default "Destroyed"))
  (bind _returnvalue (Transformation|GetActorTransform))
  (switch Utilities|FlowControl|Switch|SwitchonEEndPlayReason EndPlayReason
    (:Destroyed
      ;[0.15 0.15 0.15 0.5] Add to score
      (bind _asbp_player_controller (Utilities|Casting|CastToBP_PlayerController (Game|GetPlayerController 0)))
      (Default|AddtoPlayerScore _asbp_player_controller (Variables|/Game/Blueprints/AC_Properties.AC_Properties_C|GetHealth (Variables|Default|GetAC_Properties)))
      ;[0.15 0.15 0.15 0.5] Spawn pickup on chance
      (if (< (Math|Random|RandomFloat) 0.2)
        (Game|SpawnActorfromClass "/Game/Blueprints/Pickups/BP_LaserPickup.BP_LaserPickup_C" (Math|Transform|MakeTransform (.location _returnvalue) (.rotation _returnvalue) "1.000000,1.000000,1.000000") "Undefined" "MultiplyWithRoot" 0 "(R=0.000000,G=0.000000,B=0.000000,A=1.000000)" 0)))))

(fn ConstructionScript)