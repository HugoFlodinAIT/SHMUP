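; BP_Missile is a missile projectile actor that flies a scripted path from its spawn location.
; On BeginPlay it stores that location and starts a Timeline whose two curves drive scaled world X travel and Y offset.
; RightSideSpawn flips the sign of the Y offset, mirroring the path for either side.
; Each update sets the location directly without sweep, and the graph handles no rotation, hits or destruction.
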(event EventBeginPlay
  (Variables|Default|SetInitialLocation (Transformation|GetActorLocation))
  (bind (_direction _missilemovementy _missilemovementx) (Timeline|Timeline PlayFromStart)
    (:Update
      (Transformation|SetActorLocation (+ (Math|Vector|MakeVector (* _missilemovementx 8e+03) (* _missilemovementy (Math|Float|SelectFloat 4e+02 -4e+02 (Variables|Default|GetRightSideSpawn))) 0.0) (Variables|Default|GetInitialLocation)) false false))))

(fn ConstructionScript)