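; BP_HudClass is a HUD Blueprint that creates the player's on-screen HUD and pause menu widgets.
; On BeginPlay it calls two custom events, each creating a widget for the owning player controller and storing it in a variable.
; Both widgets go straight to the viewport, with the pause menu at a higher Z-order so it layers above the HUD.
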(event Custom|CreatePauseMenu
  (bind _returnvalue (UserInterface|CreateWidget "/Game/UI/WBP_PauseMenu.WBP_PauseMenu_C" (Game|Player|GetOwningPlayerController)))
  (bind _output_get (Variables|Default|SetPauseMenu _returnvalue))
  (UserInterface|Viewport|AddtoViewport _output_get 10))

(event Custom|CreateHudWidget
  (bind _returnvalue (UserInterface|CreateWidget "/Game/UI/WBP_HUD.WBP_HUD_C" (Game|Player|GetOwningPlayerController)))
  (bind _output_get (Variables|Default|SetHudWidget _returnvalue))
  (UserInterface|Viewport|AddtoViewport _output_get 0))

(event EventBeginPlay
  (CallFunction|CreatePauseMenu)
  (CallFunction|CreateHudWidget))

(fn ConstructionScript)