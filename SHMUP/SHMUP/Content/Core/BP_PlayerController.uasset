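; Player controller that manages the camera view, input modes, pausing and a running player score.
; BeginPlay switches to the level's first found CameraActor with UI-only input, and possession adds the global Enhanced Input mapping context.
; The pause action shows the HUD pause menu and re-pauses when already paused, otherwise resumes game-only input.
; UnpauseGame shares that resume path, which leaves menu visibility untouched.
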(event Custom|UnpauseGame
  (Game|SetGamePaused false)
  (Input|SetInputModeGameOnly self false)
  (Variables|Default|SetbShowMouseCursor false))

(event Custom|AddToPlayerScore
  (params (PointsToAdd :type Float%20%28double-precision%29))
  (Variables|Default|SetPlayerScore (+ PointsToAdd (Variables|Default|GetPlayerScore))))

(event Input|EnhancedActionEvents|EnhancedInputActionIA_PauseGame
  (params (ActionValue :type Boolean) (ElapsedSeconds :type Float%20%28double-precision%29) (TriggeredSeconds :type Float%20%28double-precision%29) (InputAction :type Input%20Action%20Object%20Reference :default "/Game/Inputs/IA_PauseGame.IA_PauseGame"))
  (:Started
    (if (Game|IsGamePaused)
      (bind _asbp_hud_class (Utilities|Casting|CastToBP_HudClass (HUD|GetHUD)))
      (Widget|SetVisibility (Variables|/Game/Core/BP_HudClass.BP_HudClass_C|GetPauseMenu _asbp_hud_class) "Visible")
      (Game|SetGamePaused true)
      (Input|SetInputModeUIOnly self (Variables|/Game/Core/BP_HudClass.BP_HudClass_C|GetPauseMenu _asbp_hud_class) "DoNotLock" true)
      (Variables|Default|SetbShowMouseCursor true)
      (else
        (Game|SetGamePaused false)
        (Input|SetInputModeGameOnly self false)
        (Variables|Default|SetbShowMouseCursor false)))))

(event EventBeginPlay
  (bind _returnvalue (Actor|GetActorOfClass "/Script/Engine.CameraActor"))
  (Game|Player|SetViewTargetwithBlend _returnvalue 0.0 "VTBlend_Linear" 0.0 false)
  (Input|SetInputModeUIOnly self 0 "DoNotLock" true)
  (Variables|Default|SetbShowMouseCursor true))

(event EventPossess
  (params (PossessedPawn :type Pawn%20Object%20Reference))
  (bind _asplayer_controller (Utilities|Casting|CastToPlayerController (Pawn|GetController PossessedPawn)))
  (Input|AddMappingContext (PlayerController|LocalPlayerSubsystems|GetEnhancedInputLocalPlayerSubsystem _asplayer_controller) "/Game/Inputs/IMC_GlobalInput.IMC_GlobalInput" 0 "(bIgnoreAllPressedKeysUntilRelease=True,bForceImmediately=False,bNotifyUserSettings=False)"))

(fn ConstructionScript)